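; Computer actor that can be hacked, turning its mesh blue and becoming interactable.
; Hacked applies both changes only on the authority; the Test event makes the same changes without that check, and Interactable's OnRep is empty.
; While Interactable, any overlap with its Box adds a new UMG_Options widget to player 0's viewport.
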(event `self.Box.OnComponentBeginOverlap`
  (params (OverlappedComponent :type "PrimitiveComponent Object Reference") (OtherActor :type "Actor Object Reference") (OtherComp :type "PrimitiveComponent Object Reference") (OtherBodyIndex :type Integer) (bFromSweep :type Boolean) (SweepResult :type "HitResult Structure (by ref)"))
  (if (`self.Interactable`)
    (bind _returnvalue (`|CreateWidget` "/Game/UMG/UMG_Options.UMG_Options_C" (`GameplayStatics.GetPlayerController` 0)))
    (`UserWidget.AddToViewport` _returnvalue 0)))

(event `Test`
  (if true
    (`PrimitiveComponent.SetMaterial` (`self.StaticMesh`) 0 "/Game/Materials/M_Blue.M_Blue")
    (set `self.Interactable` true)))

(fn `Hacked`
  (`/Engine/EditorBlueprintResources/ActorMacros.Switch Has Authority`
    (:`Authority`
      (`PrimitiveComponent.SetMaterial` (`self.StaticMesh`) 0 "/Game/Materials/M_Blue.M_Blue")
      (set `self.Interactable` true))))

(fn `OnRep_Interactable`)

(fn `UserConstructionScript`)